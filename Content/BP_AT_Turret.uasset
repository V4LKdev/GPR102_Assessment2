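; BP_AT_Turret is a turret that aims at the player's camera and periodically fires BP_AT_Projectile actors.
; Each Tick it rotates RotationPoint along the look-at rotation from CentreMuzzle to player 0's camera location.
; A Delay in the Tick chain throttles firing to about every two seconds, as it ignores re-triggers while pending.
; Projectiles spawn at the muzzle's current transform, regardless of collisions.
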(event `self.ReceiveTick`
  (params (DeltaSeconds :type "Float (single-precision)"))
  (`SceneComponent.K2_SetWorldRotation` (`self.RotationPoint`) (`KismetMathLibrary.FindLookAtRotation` (`SceneComponent.K2_GetComponentLocation` (`self.CentreMuzzle`)) (`PlayerCameraManager.GetCameraLocation` (`GameplayStatics.GetPlayerCameraManager` 0))) false false)
  (`KismetSystemLibrary.Delay` 2.0)
  (`|SpawnActorFromClass` "/Game/BP_AT_Projectile.BP_AT_Projectile_C" (`SceneComponent.K2_GetComponentToWorld` (`self.CentreMuzzle`)) "AlwaysSpawn" "MultiplyWithRoot" null null))

(fn `UserConstructionScript`)